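; AI guard that runs the BT_Guard behavior tree and shows its alert state on a status widget.
; AI perception updates write IsPlayerSensed and DetectedActor to the blackboard, clearing both when sensing fails, with no check on the sensed actor's type.
; OnStateChanged sets the widget text to "?" for Idle or Suspicious and "!" for Alert.
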(event `self.ReceiveBeginPlay`
  (`AIController.RunBehaviorTree` (`AIBlueprintHelperLibrary.GetAIController` self) "/Game/Game/AI/BehaviourTree/AIGuard/BT_Guard.BT_Guard")
  (bind _aswbp_guard_status (cast `/Game/Game/AI/WBP_GuardStatus` (`WidgetComponent.GetUserWidgetObject` (`self.StatusGuardWidget`))))
  (set `self.WBP_StatusGuard` _aswbp_guard_status))

(event `self.OnStateChanged`
  (params (NewState :type "EAIState Enum" :default "VE_IDLE"))
  (`/Game/Game/AI/WBP_GuardStatus.UpdateText` (`self.WBP_StatusGuard`) (select `EAIState` NewState :`VE_IDLE` "?" :`VE_SUSPICIOUS` "?" :`VE_ALERT` "!" :!type "Text")))

(event `self.AIPerception.OnTargetPerceptionUpdated`
  (params (Actor :type "Actor Object Reference") (Stimulus :type "AIStimulus Structure"))
  (if (`.bSuccessfullySensed` (break `AIStimulus` Stimulus))
    (`self.UpdatePlayerSensedKey` true Actor)
    (else
      (`self.UpdatePlayerSensedKey` false))))

(fn `UpdatePlayerSensedKey`
  (params (bPlayerSensed :type Boolean) (Player :type "Actor Object Reference"))
  (bind _returnvalue (`AIBlueprintHelperLibrary.GetBlackboard` (`AIBlueprintHelperLibrary.GetAIController` self)))
  (`BlackboardComponent.SetValueAsBool` _returnvalue "IsPlayerSensed" bPlayerSensed)
  (`BlackboardComponent.SetValueAsObject` _returnvalue "DetectedActor" Player))

(fn `UserConstructionScript`)