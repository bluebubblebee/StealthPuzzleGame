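; BP_RobotCharacter is a robot character that ends the attempt when it detects the player.
; Every tick it calls MakeNoise.
; On detection it prints a debug string, stops its own movement, locks input on the main player controller, then after a short delay opens the ExampleAI level.
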(event `self.ReceiveTick`
  (params (DeltaSeconds :type "Float (single-precision)"))
  (`self.MakeNoise` 1.0 null))

(event `OnDetect`
  (`KismetSystemLibrary.PrintString` "OnDetectPlayer")
  (`MovementComponent.StopMovementImmediately` (`self.CharacterMovement`))
  (bind _asbp_main_player_controller (cast `/Game/Game/Blueprints/BP_MainPlayerController` (`GameplayStatics.GetPlayerController` 0)))
  (`UntitledLittleThiefPlayerController.LockInput` _asbp_main_player_controller)
  (`KismetSystemLibrary.Delay` 5.0)
  (`GameplayStatics.OpenLevel` "ExampleAI"))

(fn `UserConstructionScript`
  (`parent.UserConstructionScript`))