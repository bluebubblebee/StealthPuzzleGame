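; BP_SwitchPlatform_2_0 is a Level 2 switch platform that animates its screen when switched on or off.
; BeginPlay puts a dynamic material instance on the Screen component and sets its Alpha parameter to zero.
; OnSwitchon and OnSwitchOff each play an electronic click at the world origin and run their own timeline from the start to drive that Alpha.
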(event `self.ReceiveBeginPlay`
  (bind _screen (`self.Screen`))
  ;[1 1 1] Initialize Screen Material
  (bind _returnvalue (`PrimitiveComponent.CreateDynamicMaterialInstance` _screen 0 (`PrimitiveComponent.GetMaterial` _screen 0) "None"))
  (bind _output_get (set `self.ScreenMaterialInstance` _returnvalue))
  (`PrimitiveComponent.SetMaterial` (`self.Screen`) 0 _output_get)
  (`MaterialInstanceDynamic.SetScalarParameterValue` _output_get "Alpha" 0.0))

(event `self.OnSwitchOff`
  (`GameplayStatics.PlaySoundAtLocation` "/Game/Game/Audio/Click_Electronic_00.Click_Electronic_00" (0.0 0.0 0.0) (struct) 1.0 1.0 0.0 null null null)
  (bind (_direction _alpha) (`Timeline|Timeline_0` :!via `PlayFromStart`)
    (:`Update`
      (`MaterialInstanceDynamic.SetScalarParameterValue` (`self.ScreenMaterialInstance`) "Alpha" _alpha))))

(event `self.OnSwitchOn`
  (`GameplayStatics.PlaySoundAtLocation` "/Game/Game/Audio/Click_Electronic_00.Click_Electronic_00" (0.0 0.0 0.0) (struct) 1.0 1.0 0.0 null null null)
  (bind (_direction _alpha) (`Timeline|Timeline_1` :!via `PlayFromStart`)
    (:`Update`
      (`MaterialInstanceDynamic.SetScalarParameterValue` (`self.ScreenMaterialInstance`) "Alpha" _alpha))))

(fn `UserConstructionScript`)