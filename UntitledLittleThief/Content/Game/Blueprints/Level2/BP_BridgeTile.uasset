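; BP_BridgeTile is a Level 2 bridge tile that switches between hidden and shown states.
; It starts with Wall2, Wall3 and its Collision component switched off on BeginPlay.
; OnTileShown makes both walls visible, including their children, and enables query and physics collision.
; OnTileHidden hides both walls without propagating to children and disables the collision again.
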(event `self.ReceiveBeginPlay`
  ;[1 1 1] Hide walls and collision
  (`|ExecutionSequence`
    (:`then_0`
      (`SceneComponent.SetVisibility` (`self.Wall2`) false false))
    (:`then_1`
      (`SceneComponent.SetVisibility` (`self.Wall3`) false false))
    (:`then_2`
      (`PrimitiveComponent.SetCollisionEnabled` (`self.Collision`) "NoCollision"))))

(event `self.OnTileShown`
  (`|ExecutionSequence`
    (:`then_0`
      (`SceneComponent.SetVisibility` (`self.Wall3`) true true))
    (:`then_1`
      (`SceneComponent.SetVisibility` (`self.Wall2`) true true))
    (:`then_2`
      (`PrimitiveComponent.SetCollisionEnabled` (`self.Collision`) "QueryAndPhysics"))))

(event `self.OnTileHidden`
  (`|ExecutionSequence`
    (:`then_0`
      (`SceneComponent.SetVisibility` (`self.Wall3`) false false))
    (:`then_1`
      (`SceneComponent.SetVisibility` (`self.Wall2`) false false))
    (:`then_2`
      (`PrimitiveComponent.SetCollisionEnabled` (`self.Collision`) "NoCollision"))))

(fn `UserConstructionScript`)