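; BP_LockedDoor is a Level 2 door that stays blocked until an OnOpenDoor event opens it after a caller-supplied delay.
; On opening, it disables the box collision and plays two timelines that move the bottom and top parts along Z.
; The top part is hidden shortly after the animations start.
; The door has no overlap or tick logic, so opening depends entirely on that event being called.
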(event `self.OnOpenDoor`
  (params (Delay :type "Float (single-precision)"))
  (`KismetSystemLibrary.Delay` Delay)
  (`PrimitiveComponent.SetCollisionEnabled` (`self.BoxCollision`) "NoCollision")
  (`|ExecutionSequence`
    (:`then_0`
      (bind (_direction _zvalue) (`Timeline|BottomDoorAnimation` :!via `PlayFromStart`)
        (:`Update`
          (`SceneComponent.K2_SetRelativeLocation` (`self.BottomPart`) (`KismetMathLibrary.MakeVector` 0.0 0.0 _zvalue) false false))))
    (:`then_1`
      (bind (_direction_2 _zvalue_2) (`Timeline|TopDoorAnimation` :!via `PlayFromStart`)
        (:`Update`
          (`SceneComponent.K2_SetRelativeLocation` (`self.TopPart`) (`KismetMathLibrary.MakeVector` 0.0 0.0 _zvalue_2) false false))))
    (:`then_2`
      (`KismetSystemLibrary.Delay` 0.7)
      (`SceneComponent.SetVisibility` (`self.TopPart`) false false))))

(fn `UserConstructionScript`)